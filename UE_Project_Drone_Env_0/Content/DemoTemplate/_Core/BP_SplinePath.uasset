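; Spline path actor that draws a route as decals, built entirely in the construction script with no runtime logic.
; Each spline point gets a marker decal, and each gap between neighboring points gets a direction decal at its midpoint, yawed along the segment.
; Segment decals stretch with point distance minus a fixed margin, widen their projection depth with height difference, and use a dynamic M_D_Direction material whose Size parameter matches the length.
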(fn `UserConstructionScript`
  (bind _spline (`self.Spline`))
  (bind _returnvalue (`SplineComponent.GetNumberOfSplinePoints` _spline))
  (for _index (range (+ _returnvalue 1))
    (bind _returnvalue_2 (`SplineComponent.GetLocationAtSplinePoint` _spline _index "Local"))
    (`AddComponent|NODE_AddDecalComponent-0` :`RelativeTransform` (`KismetMathLibrary.MakeTransform` _returnvalue_2 (struct :`Pitch` 90.0)))
    (if (< _index (- _returnvalue 1))
      (bind _returnvalue_3 (`KismetMaterialLibrary.CreateDynamicMaterialInstance` "/Game/DemoTemplate/_Core/M_D_Direction.M_D_Direction"))
      (bind _returnvalue_4 (`SplineComponent.GetLocationAtSplinePoint` (`self.Spline`) (+ _index 1) "Local"))
      (bind _returnvalue_5 (- _returnvalue_2 _returnvalue_4))
      (bind _returnvalue_6 (/ (- (`KismetMathLibrary.VSize` _returnvalue_5) 200.0) 200.0))
      (`MaterialInstanceDynamic.SetScalarParameterValue` _returnvalue_3 "Size" _returnvalue_6)
      (bind (_returnvalue_roll _returnvalue_pitch _returnvalue_yaw) (`KismetMathLibrary.BreakRotator` (`KismetMathLibrary.FindLookAtRotation` _returnvalue_2 _returnvalue_4)))
      (bind _returnvalue_7 (`AddComponent|NODE_AddDecalComponent-1` :`RelativeTransform` (`KismetMathLibrary.MakeTransform` (`KismetMathLibrary.VLerp` _returnvalue_2 _returnvalue_4 0.5) (`KismetMathLibrary.MakeRotator` 0.0 90.0 (+ _returnvalue_yaw -90.0)) (`KismetMathLibrary.MakeVector` (+ (/ (`KismetMathLibrary.Abs` (.z _returnvalue_5)) 200.0) 0.5) _returnvalue_6 0.1))))
      (`DecalComponent.SetDecalMaterial` _returnvalue_7 _returnvalue_3))))