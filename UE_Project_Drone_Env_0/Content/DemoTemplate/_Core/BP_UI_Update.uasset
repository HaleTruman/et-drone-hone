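; Trigger actor that shows and hides editor-style UI panels (Details, Content, Outliner, Transform) in the demo template.
; On begin overlap it toggles each flagged panel on through the UI held by BP_GM_Template, and on end overlap toggles the same panels off.
; Per-panel booleans select which panels each instance controls.
; The overlapping actor is not filtered, so any overlap triggers the change.
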(event `self.ReceiveActorBeginOverlap`
  (params (OtherActor :type "Actor Object Reference"))
  (bind _asbp_gm_template (cast `/Game/DemoTemplate/_Core/BP_GM_Template` (`GameplayStatics.GetGameMode`)))
  (`|ExecutionSequence`
    (:`then_0`
      (if (`self.Show Details`)
        (bind _ui (`/Game/DemoTemplate/_Core/BP_GM_Template.UI` _asbp_gm_template))
        (`/Game/DemoTemplate/_Core/UI_InGame.Toggle Details` _ui true)))
    (:`then_1`
      (if (`self.Show Content`)
        (`/Game/DemoTemplate/_Core/UI_InGame.Toggle Content` _ui true)))
    (:`then_2`
      (if (`self.Show Outliner`)
        (`/Game/DemoTemplate/_Core/UI_InGame.Toggle Outliner` _ui true)))
    (:`then_3`
      (if (`self.Show Transform`)
        (`/Game/DemoTemplate/_Core/UI_InGame.Toggle Transform` _ui true)))))

(event `self.ReceiveActorEndOverlap`
  (params (OtherActor :type "Actor Object Reference"))
  (bind _asbp_gm_template (cast `/Game/DemoTemplate/_Core/BP_GM_Template` (`GameplayStatics.GetGameMode`)))
  (`|ExecutionSequence`
    (:`then_0`
      (if (`self.Show Details`)
        (bind _ui (`/Game/DemoTemplate/_Core/BP_GM_Template.UI` _asbp_gm_template))
        (`/Game/DemoTemplate/_Core/UI_InGame.Toggle Details` _ui false)))
    (:`then_1`
      (if (`self.Show Content`)
        (`/Game/DemoTemplate/_Core/UI_InGame.Toggle Content` _ui false)))
    (:`then_2`
      (if (`self.Show Outliner`)
        (`/Game/DemoTemplate/_Core/UI_InGame.Toggle Outliner` _ui false)))
    (:`then_3`
      (if (`self.Show Transform`)
        (`/Game/DemoTemplate/_Core/UI_InGame.Toggle Transform` _ui false)))))

(fn `UserConstructionScript`)