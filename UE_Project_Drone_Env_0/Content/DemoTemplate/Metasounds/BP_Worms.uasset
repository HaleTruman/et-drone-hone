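; Singing worm actor for a MetaSound demo that rises, opens its mouth and gets louder as the player looks up while inside its capsule.
; On BeginPlay it creates a dynamic singer material and sends its Pitch value to the audio's MidiIn parameter.
; Capsule overlaps toggle a per-tick update that maps camera pitch to one clamped value driving mouth scale, mesh height and volume.
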(event `self.ReceiveBeginPlay`
  (bind _returnvalue (`PrimitiveComponent.CreateDynamicMaterialInstance` (`self.StaticMesh`) 0 "/Game/DemoTemplate/Metasounds/M_Singer.M_Singer" "None"))
  (set `self.NewVar` _returnvalue)
  (`AudioParameterControllerInterface.SetFloatParameter` (`self.Audio`) "MidiIn" (`self.Pitch`)))

(event `self.ReceiveTick`
  (params (DeltaSeconds :type "Float (single-precision)"))
  (bind _returnvalue (`KismetMathLibrary.FClamp` (+ (* (/ (`KismetMathLibrary.NormalizeAxis` (.pitch (`Controller.GetControlRotation` (`GameplayStatics.GetPlayerController` 0)))) 40.0) 3.0) 0.4) 0.0 1.0))
  (if (`self.Update Pitch`)
    (`MaterialInstanceDynamic.SetScalarParameterValue` (`self.NewVar`) "Mouth Scale" _returnvalue)
    (`SceneComponent.K2_SetRelativeLocation` (`self.StaticMesh`) (`KismetMathLibrary.MakeVector` 0.0 0.0 (`KismetMathLibrary.Lerp` -150.0 45.0 _returnvalue)) false false)
    (`AudioComponent.SetVolumeMultiplier` (`self.Audio`) _returnvalue)))

(event `self.Capsule.OnComponentBeginOverlap`
  (params (OverlappedComponent :type "PrimitiveComponent Object Reference") (OtherActor :type "Actor Object Reference") (OtherComp :type "PrimitiveComponent Object Reference") (OtherBodyIndex :type Integer) (bFromSweep :type Boolean) (SweepResult :type "HitResult Structure (by ref)"))
  (set `self.Update Pitch` true))

(event `self.Capsule.OnComponentEndOverlap`
  (params (OverlappedComponent :type "PrimitiveComponent Object Reference") (OtherActor :type "Actor Object Reference") (OtherComp :type "PrimitiveComponent Object Reference") (OtherBodyIndex :type Integer))
  (set `self.Update Pitch` false))

(fn `UserConstructionScript`)